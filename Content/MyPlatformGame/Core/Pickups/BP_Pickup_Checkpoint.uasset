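; Checkpoint pickup that records its location in the platform game mode as the last checkpoint when picked up.
; On BeginPlay it caches BP_PlatformGameMode and registers itself in that mode's Checkpoints array.
; PickupEvent calls the parent logic, stores the location, then unhides every registered checkpoint and hides itself, so the most recently collected one is hidden.
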(event EventBeginPlay
  (bind _asbp_platform_game_mode (Utilities|Casting|CastToBP_PlatformGameMode (Game|GetGameMode)))
  (bind _output_get (Variables|Default|SetMyGameMode _asbp_platform_game_mode))
  (Utilities|Array|Add (Variables|/Game/MyPlatformGame/Core/Framework/BP_PlatformGameMode.BP_PlatformGameMode_C|GetCheckpoints _output_get) self))

(fn ConstructionScript
  (|CallParentFunction))

(fn PickupEvent
  (params (OverlappingActor :type Actor%20Object%20Reference))
  (|CallParentFunction OverlappingActor)
  (Variables|/Game/MyPlatformGame/Core/Framework/BP_PlatformGameMode.BP_PlatformGameMode_C|SetLastCheckpointLocation (Variables|Default|GetMyGameMode) (Transformation|GetActorLocation))
  (for _array_element (Variables|/Game/MyPlatformGame/Core/Framework/BP_PlatformGameMode.BP_PlatformGameMode_C|GetCheckpoints (Variables|Default|GetMyGameMode))
    (Rendering|SetActorHiddenInGame _array_element false))
  (Rendering|SetActorHiddenInGame true))