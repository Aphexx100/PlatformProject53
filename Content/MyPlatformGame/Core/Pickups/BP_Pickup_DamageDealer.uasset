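; BP_Pickup_DamageDealer is a harmful pickup that damages the hero who collects it.
; It extends a parent pickup's PickupEvent, applying a fixed amount of damage to an overlapping BP_HeroBase and then destroying itself.
; Any other overlapping actor only triggers an on-screen debug message.
; BeginPlay caches the first player's BP_PlatformerPlayerState, though the pickup logic here does not use it.
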(event EventBeginPlay
  (bind _asbp_platformer_player_state (Utilities|Casting|CastToBP_PlatformerPlayerState (Game|GetPlayerState 0)))
  (Variables|Default|SetMyPlayerState _asbp_platformer_player_state))

(fn ConstructionScript
  (|CallParentFunction))

(fn PickupEvent
  (params (OverlappingActor :type Actor%20Object%20Reference))
  (|CallParentFunction OverlappingActor)
  (bind _asbp_hero_base (Utilities|Casting|CastToBP_HeroBase OverlappingActor)
    (:then
      (Game|Damage|ApplyDamage _asbp_hero_base 25.0 0 self)
      (Actor|DestroyActor))
    (:CastFailed
      (Development|PrintString "I wanted to damage hero but found no hero: BP_Pickup_Damagedealer" true true "(R=1.000000,G=0.057227,B=0.000000,A=1.000000)" 1e+01))))