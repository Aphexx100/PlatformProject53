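; BP_SecurityCamDriver is a trigger volume that switches the player's view to an external security camera that tracks them.
; Box overlap sets the view target to ExternalCam and starts a fast looping timer that turns it toward the stored actor.
; Leaving returns the view to that actor and clears the timer.
; The player check matches "HeroBase" in the class display name, avoiding a cast reference.
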(event OnComponentBeginOverlap(Box)
  (params (OverlappedComponent :type Primitive%20Component%20Object%20Reference) (OtherActor :type Actor%20Object%20Reference) (OtherComp :type Primitive%20Component%20Object%20Reference) (OtherBodyIndex :type Integer) (bFromSweep :type Boolean) (SweepResult :type Hit%20Result%20Structure%20%28by%20ref%29))
  (Utilities|TestforPlayerWithoutReference OtherActor
    (:true
      (Game|Player|SetViewTargetwithBlend (Game|GetPlayerController 0) (Variables|Default|GetExternalCam) 0.0 "VTBlend_Linear" 0.0 false)
      (bind _returnvalue (Utilities|Time|SetTimerbyFunctionName 0 "ObservePlayer" 0.01 true))
      (Variables|Default|SetObserveTimer _returnvalue))))

(event OnComponentEndOverlap(Box)
  (params (OverlappedComponent :type Primitive%20Component%20Object%20Reference) (OtherActor :type Actor%20Object%20Reference) (OtherComp :type Primitive%20Component%20Object%20Reference) (OtherBodyIndex :type Integer))
  (Utilities|TestforPlayerWithoutReference OtherActor
    (:true
      (Game|Player|SetViewTargetwithBlend (Game|GetPlayerController 0) OtherActor 0.0 "VTBlend_Linear" 0.0 false)
      (Utilities|Time|ClearandInvalidateTimerbyHandle (Variables|Default|GetObserveTimer)))))

(event Custom|ObservePlayer
  (Transformation|SetActorRotation (Variables|Default|GetExternalCam) (Math|Rotator|FindLookatRotation (Transformation|GetActorLocation (Variables|Default|GetExternalCam)) (Transformation|GetActorLocation (Variables|Default|GetMyOverlappedActor)))))

(fn ConstructionScript)