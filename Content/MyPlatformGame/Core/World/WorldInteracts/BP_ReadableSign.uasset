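; Readable sign actor that switches the player's view to itself when the hero enters its trigger box.
; Construction script applies configurable text and size to a TextRender.
; Box overlap identifies the hero by a "HeroBase" substring in the class display name, avoiding a cast, then blends the camera to the sign.
; Right mouse returns the view to the player character; end overlap switches it to whichever actor left, without the hero check.
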(event OnComponentBeginOverlap(Box)
  (params (OverlappedComponent :type Primitive%20Component%20Object%20Reference) (OtherActor :type Actor%20Object%20Reference) (OtherComp :type Primitive%20Component%20Object%20Reference) (OtherBodyIndex :type Integer) (bFromSweep :type Boolean) (SweepResult :type Hit%20Result%20Structure%20%28by%20ref%29))
  (Utilities|TestforPlayerWithoutReference OtherActor
    (:true
      (Game|Player|SetViewTargetwithBlend (Game|GetPlayerController 0) self 2.0 "VTBlend_Linear" 0.0 false))))

(event OnComponentEndOverlap(Box)
  (params (OverlappedComponent :type Primitive%20Component%20Object%20Reference) (OtherActor :type Actor%20Object%20Reference) (OtherComp :type Primitive%20Component%20Object%20Reference) (OtherBodyIndex :type Integer))
  (Game|Player|SetViewTargetwithBlend (Game|GetPlayerController 0) OtherActor 0.0 "VTBlend_Linear" 0.5 false))

(event EventBeginPlay)

(event Collision|EventActorBeginOverlap
  (params (OtherActor :type Actor%20Object%20Reference)))

(event EventTick
  (params (DeltaSeconds :type Float%20%28single-precision%29)))

(event Input|MouseEvents|RightMouseButton
  (params (Key :type Key%20Structure :default "None"))
  (:Pressed
    (Game|Player|SetViewTargetwithBlend (Game|GetPlayerController 0) (Game|GetPlayerCharacter 0) 0.0 "VTBlend_Linear" 0.5 false)))

(fn ConstructionScript
  (bind _textrender (Variables|Default|GetTextRender))
  (Rendering|Components|TextRender|SetText _textrender (Variables|Default|GetMyText))
  (Rendering|Components|TextRender|SetWorldSize _textrender (Variables|Default|GetTextSize)))