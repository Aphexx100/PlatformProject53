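; Base enemy Blueprint for a moving hazard that deals heavy point damage when its mesh overlaps the player character.
; Movement starts at BeginPlay or on trigger-sphere overlap, with timeline play rates derived from a travel time.
; A timeline either lerps the mesh to a target offset, reversing at each end to oscillate, or drives it along a spline.
; The construction script applies the exposed mesh, trigger placement and spline loop setting.
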(event OnComponentBeginOverlap(Sphere)
  (params (OverlappedComponent :type Primitive%20Component%20Object%20Reference) (OtherActor :type Actor%20Object%20Reference) (OtherComp :type Primitive%20Component%20Object%20Reference) (OtherBodyIndex :type Integer) (bFromSweep :type Boolean) (SweepResult :type Hit%20Result%20Structure%20%28by%20ref%29))
  ;[0 0 0] Start Timeline by trigger
  (if (and (Variables|Trigger|GetMoveOnTrigger) (!= OtherActor self))
    (if (Variables|SplineMovement|GetUseSplineMovement)
      (CallFunction|PlaySplineMovement)
      (else
        (bind (_direction _0_1) (Timeline|MovementDriver Play)
          (:Update
            ;[0 0 0] Move to target location
            (Transformation|SetRelativeLocation (Variables|Default|GetCone) (Math|Vector|Lerp(Vector) "0, 0, 0" (Variables|Movement|GetTargetLocation) _0_1) false false))
          (:Finished
            ;[0 0 0] Oscillating Movement
            (switch Utilities|FlowControl|Switch|SwitchonETimelineDirection _direction
              (:Forward
                (CallFunction|Reverse))
              (:Backward
                (CallFunction|Replay)))))))))

(event OnComponentBeginOverlap(Cone)
  (params (OverlappedComponent :type Primitive%20Component%20Object%20Reference) (OtherActor :type Actor%20Object%20Reference) (OtherComp :type Primitive%20Component%20Object%20Reference) (OtherBodyIndex :type Integer) (bFromSweep :type Boolean) (SweepResult :type Hit%20Result%20Structure%20%28by%20ref%29))
  ;[0 0 0] Deal Damage
  (if (== OtherActor (Game|GetPlayerCharacter 0))
    (Game|Damage|ApplyPointDamage OtherActor 1e+03 (- (Transformation|GetActorForwardVector OtherActor) (Transformation|GetActorLocation)) SweepResult 0 self)))

(event Custom|Reverse
  (bind (_direction _0_1) (Timeline|MovementDriver ReverseFromEnd)
    (:Update
      ;[0 0 0] Move to target location
      (Transformation|SetRelativeLocation (Variables|Default|GetCone) (Math|Vector|Lerp(Vector) "0, 0, 0" (Variables|Movement|GetTargetLocation) _0_1) false false))
    (:Finished
      ;[0 0 0] Oscillating Movement
      (switch Utilities|FlowControl|Switch|SwitchonETimelineDirection _direction
        (:Forward
          (CallFunction|Reverse))
        (:Backward
          (CallFunction|Replay))))))

(event Custom|Replay
  (bind (_direction _0_1) (Timeline|MovementDriver PlayFromStart)
    (:Update
      ;[0 0 0] Move to target location
      (Transformation|SetRelativeLocation (Variables|Default|GetCone) (Math|Vector|Lerp(Vector) "0, 0, 0" (Variables|Movement|GetTargetLocation) _0_1) false false))
    (:Finished
      ;[0 0 0] Oscillating Movement
      (switch Utilities|FlowControl|Switch|SwitchonETimelineDirection _direction
        (:Forward
          (CallFunction|Reverse))
        (:Backward
          (CallFunction|Replay))))))

(event Custom|PlaySplineMovement
  (bind _spline (Variables|Default|GetSpline))
  ;[0 0 0] Move Along Spline
  (bind _0_1 (Timeline|SplineMovementDriver Play)
    (:Update
      (Transformation|SetWorldTransform (Variables|Default|GetCone) (Math|Transform|MakeTransform (Spline|GetLocationatDistanceAlongSpline _spline (Math|Float|Lerp 0.0 (Spline|GetSplineLength (Variables|Default|GetSpline)) _0_1) "World") (Spline|GetRotationatDistanceAlongSpline _spline (Math|Float|Lerp 0.0 (Spline|GetSplineLength (Variables|Default|GetSpline)) _0_1) "Local") "1.000000,1.000000,1.000000") false false))))

(event EventBeginPlay
  ;[0 0 0] Set Play Conditions
  (Components|Timeline|SetPlayRate (Variables|Default|GetMovementDriver) (/ 1.0 (Variables|Movement|GetTimeToReachTarget)))
  (if (not (Variables|Trigger|GetMoveOnTrigger))
    (if (Variables|SplineMovement|GetUseSplineMovement)
      (CallFunction|PlaySplineMovement)
      (else
        (bind (_direction _0_1) (Timeline|MovementDriver Play)
          (:Update
            ;[0 0 0] Move to target location
            (Transformation|SetRelativeLocation (Variables|Default|GetCone) (Math|Vector|Lerp(Vector) "0, 0, 0" (Variables|Movement|GetTargetLocation) _0_1) false false))
          (:Finished
            ;[0 0 0] Oscillating Movement
            (switch Utilities|FlowControl|Switch|SwitchonETimelineDirection _direction
              (:Forward
                (CallFunction|Reverse))
              (:Backward
                (CallFunction|Replay)))))))))

(fn ConstructionScript
  (bind _sphere (Variables|Default|GetSphere))
  ;[0 0 0] Set Trigger Location and Radius
  (Components|Sphere|SetSphereRadius _sphere (Variables|Trigger|GetTriggerSphereRadius) true)
  (Transformation|SetRelativeLocation _sphere (Variables|Trigger|GetTriggerSphereLocation) false false)
  ;[0 0 0] Handle Spline
  (Spline|SetClosedLoop (Variables|Default|GetSpline) (Variables|SplineMovement|GetClosedLoop) true)
  (Components|StaticMesh|SetStaticMesh (Variables|Default|GetCone) (Variables|Visual|GetMyVisual)))