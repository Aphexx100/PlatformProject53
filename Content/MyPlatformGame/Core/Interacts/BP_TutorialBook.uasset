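; BP_TutorialBook is an interactable book that opens and closes a journal widget for the player.
; Its InteractFunction event uses a FlipFlop: one interaction creates WBP_Journal, shows the cursor and switches to Game and UI input.
; The next interaction removes the widget, hides the cursor and restores game-only input, toggling the Hero's IsInMenu flag alongside.
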(event EventInteractFunction
  (params (MessageString :type String) (Hero :type BP%20Hero%20Base%20Object%20Reference))
  (bind _returnvalue (Game|GetPlayerController 0))
  (bind _returnvalue_2 (Game|GetPlayerController 0))
  (Utilities|FlowControl|FlipFlop
    (:A
      (bind _returnvalue_3 (UserInterface|CreateWidget "/Game/MyPlatformGame/Art/HUD/Journal/WBP_Journal_1.WBP_Journal_1_C"))
      (UserInterface|Viewport|AddtoViewport _returnvalue_3 0)
      (Variables|/Script/Engine.PlayerController|SetbShowMouseCursor _returnvalue_2 true)
      (Variables|/Game/MyPlatformGame/Core/Characters/Player/BP_HeroBase.BP_HeroBase_C|SetIsInMenu Hero true)
      (Input|SetInputModeGameandUI _returnvalue_2 0 "DoNotLock" true false))
    (:B
      (Widget|RemovefromParent _returnvalue_3)
      (Variables|/Script/Engine.PlayerController|SetbShowMouseCursor _returnvalue false)
      (Input|SetInputModeGameOnly _returnvalue false)
      (Variables|/Game/MyPlatformGame/Core/Characters/Player/BP_HeroBase.BP_HeroBase_C|SetIsInMenu Hero false))))

(fn ConstructionScript)