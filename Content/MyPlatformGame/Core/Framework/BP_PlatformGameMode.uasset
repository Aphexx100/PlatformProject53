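; Platformer game mode that manages the starting checkpoint, player death and respawn, and new-game resets.
; BeginPlay stores the PlayerStart location as the last checkpoint and caches the player state.
; PlayerDeath fades the camera out, then replaces the pawn with a new BP_HeroBase, loads the saved game through the player state, possesses the hero and fades back in.
; StartNewGame returns the character to PlayerStart and clears the checkpoint list.
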(event EventPlayerDeath
  (params (PlayerBlueprint :type BP%20Hero%20Base%20Object%20Reference))
  (Utilities|FlowControl|Sequence
    (:then_0
      (CameraFades|StartCameraFade :self (Variables|/Script/Engine.PlayerController|GetPlayerCameraManager (Game|GetPlayerController 0)) :ToAlpha 1.0 :Duration (Variables|Default|GetDeathFadeDuration) :bHoldWhenFinished true))
    (:then_1
      (Utilities|FlowControl|Delay (Variables|Default|GetDeathFadeDuration))
      (Actor|DestroyActor PlayerBlueprint)
      (bind _returnvalue (Game|SpawnActorfromClass "/Game/MyPlatformGame/Core/Characters/Player/BP_HeroBase.BP_HeroBase_C" (Math|Transform|MakeTransform "0, 0, 0" "0, 0, 0" "1.000000,1.000000,1.000000") "Undefined" "MultiplyWithRoot" 0 0))
      (Default|LoadGame (Variables|Default|GetMyPlayerState))
      (Pawn|Possess (Game|GetPlayerController 0) _returnvalue))
    (:then_2
      (Utilities|FlowControl|Delay (Variables|Default|GetDeathFadeDuration))
      (CameraFades|StartCameraFade :self (Variables|/Script/Engine.PlayerController|GetPlayerCameraManager (Game|GetPlayerController 0)) :FromAlpha 1.0 :ToAlpha 0.0 :Duration (Variables|Default|GetDeathFadeDuration) :bHoldWhenFinished true))))

(event EventBeginPlay
  ;[1 0 0] SetPlayerStartAsFirstCheckpoint
  (bind _returnvalue (Actor|GetActorOfClass "/Script/Engine.PlayerStart"))
  (Utilities|IsValid _returnvalue
    (:Is%20Valid
      (Variables|Default|SetLastCheckpointLocation (Transformation|GetActorLocation _returnvalue))
      (Variables|Default|SetMyPlayerState (.AsBP%20Platformer%20Player%20State (Utilities|Casting|CastToBP_PlatformerPlayerState (Game|GetPlayerState 0)))))))

(fn ConstructionScript)

(fn StartNewGame
  (bind _returnvalue (Actor|GetActorOfClass "/Script/Engine.PlayerStart"))
  (Transformation|SetActorLocation (Game|GetPlayerCharacter 0) (Transformation|GetActorLocation _returnvalue) false false)
  (Utilities|Array|Clear (Variables|Default|GetCheckpoints)))