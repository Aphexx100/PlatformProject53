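; Player state for a platformer that tracks collected coins and player health and handles saving and loading game progress.
; Saving reuses or creates a BP_SaveGame_1, records health, coins, max jumps, transform and hidden state of "Saveable"-tagged actors, then writes asynchronously and shows an autosave widget.
; Loading restores actor visibility and coins, passing health, jumps and transform to the given hero through LoadSaveGameMessage.
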(event Custom|SaveTheGame
  (params (SaveSlotName :type String))
  ;[0.01103 1 0] SaveGame
  (bind _returnvalue (SaveGame|LoadGamefromSlot SaveSlotName))
  (bind _asbp_save_game_1 (Utilities|Casting|CastToBP_SaveGame_1 _returnvalue)
    (:then
      (Variables|Default|SetMySaveGame _asbp_save_game_1))
    (:CastFailed
      (bind _returnvalue_2 (SaveGame|CreateSaveGameObject "/Game/MyPlatformGame/Core/Savegames/BP_SaveGame_1.BP_SaveGame_1_C"))
      (Variables|Default|SetMySaveGame _returnvalue_2)))
  (CallFunction|SaveGameSetter)
  (|AsyncSaveGametoSlot (Variables|Default|GetMySaveGame) SaveSlotName
    (:Completed
      ;;[1 1 1] Move to Autosave BP
      (bind _returnvalue_3 (UserInterface|CreateWidget "/Game/MyPlatformGame/Core/Savegames/WBP_AutosaveNote.WBP_AutosaveNote_C"))
      (UserInterface|Viewport|AddtoViewport _returnvalue_3 0))))

(event Custom|LoadTheGame
  (params (SlotName :type String) (NewHero :type BP%20Hero%20Base%20Object%20Reference))
  ;[0.01103 1 0] LoadGame
  (bind _returnvalue (SaveGame|LoadGamefromSlot SlotName))
  (bind _asbp_save_game_1 (Utilities|Casting|CastToBP_SaveGame_1 _returnvalue))
  (CallFunction|LoadItemsfromSave _asbp_save_game_1 NewHero))

(event EventBeginPlay
  (bind _asbp_hero_base (Utilities|Casting|CastToBP_HeroBase (Game|GetPlayerCharacter 0)))
  (Variables|Default|SetMyPlayer _asbp_hero_base))

(event EventCoinCounter
  (params (CoinActor :type Actor%20Object%20Reference))
  (bind _output_get (Variables|Default|SetCollectedCoins (+ (Variables|Default|GetCollectedCoins) 1)))
  (Development|PrintString (Utilities|String|Append (Utilities|String|ToString(Integer) _output_get) " Coin amount printed in BP_PlatformerPlayerState")))

(event EventSendPlayerHealth
  (params (CurrentPlayerHealth :type Float%20%28double-precision%29))
  (Variables|Default|SetCurrentHealth CurrentPlayerHealth))

(fn ConstructionScript)

(fn SaveGameSetter
  (bind _outactors (Actor|GetAllActorswithTag "Saveable"))
  (for _array_element _outactors
    (Utilities|Map|Add (Variables|/Game/MyPlatformGame/Core/Savegames/BP_SaveGame_1.BP_SaveGame_1_C|GetPickupVisibilities (Variables|Default|GetMySaveGame)) _array_element (Variables|/Script/Engine.Actor|GetbHidden _array_element)))
  (Variables|/Game/MyPlatformGame/Core/Savegames/BP_SaveGame_1.BP_SaveGame_1_C|SetHealth (Variables|Default|GetMySaveGame) (Variables|/Game/MyPlatformGame/Core/Characters/Player/BP_HeroBase.BP_HeroBase_C|GetPlayerHealth (Variables|Default|GetMyPlayer)))
  (Variables|/Game/MyPlatformGame/Core/Savegames/BP_SaveGame_1.BP_SaveGame_1_C|SetCoins (Variables|Default|GetMySaveGame) (Variables|Default|GetCollectedCoins))
  (Variables|/Game/MyPlatformGame/Core/Savegames/BP_SaveGame_1.BP_SaveGame_1_C|SetJumpMaxCount (Variables|Default|GetMySaveGame) (Variables|/Script/Engine.Character|GetJumpMaxCount (Variables|Default|GetMyPlayer)))
  (Variables|/Game/MyPlatformGame/Core/Savegames/BP_SaveGame_1.BP_SaveGame_1_C|SetTransform (Variables|Default|GetMySaveGame) (Transformation|GetActorTransform (Variables|Default|GetMyPlayer)))
  (return))

(fn LoadItemsfromSave
  (params (SaveGame :type BP%20Save%20Game%201%20Object%20Reference) (NewHero :type BP%20Hero%20Base%20Object%20Reference))
  (bind _outactors (Actor|GetAllActorswithTag "Saveable"))
  (for _array_element _outactors
    (Rendering|SetActorHiddenInGame _array_element (.Value (Utilities|Map|Find (Variables|/Game/MyPlatformGame/Core/Savegames/BP_SaveGame_1.BP_SaveGame_1_C|GetPickupVisibilities SaveGame) _array_element))))
  (Class|BPIPlayer|LoadSaveGame(Message) NewHero (Variables|/Game/MyPlatformGame/Core/Savegames/BP_SaveGame_1.BP_SaveGame_1_C|GetHealth SaveGame) (Variables|/Game/MyPlatformGame/Core/Savegames/BP_SaveGame_1.BP_SaveGame_1_C|GetJumpMaxCount SaveGame) (Variables|/Game/MyPlatformGame/Core/Savegames/BP_SaveGame_1.BP_SaveGame_1_C|GetTransform SaveGame))
  (Variables|Default|SetCollectedCoins (Variables|/Game/MyPlatformGame/Core/Savegames/BP_SaveGame_1.BP_SaveGame_1_C|GetCoins SaveGame)))