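; Elevator platform that moves its mesh between the origin and a Target relative offset, starting on BeginPlay or, with StartOnContact, on overlap.
; The PlatformDriver timeline drives a position lerp, with play rate derived from TimeToReachTarget.
; PlayInLoop ping-pongs the timeline at each end.
; Ending overlap always reverses travel and suppresses looping until the next overlap begins.
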(event OnComponentBeginOverlap(Collision)
  (params (OverlappedComponent :type Primitive%20Component%20Object%20Reference) (OtherActor :type Actor%20Object%20Reference) (OtherComp :type Primitive%20Component%20Object%20Reference) (OtherBodyIndex :type Integer) (bFromSweep :type Boolean) (SweepResult :type Hit%20Result%20Structure%20%28by%20ref%29))
  (Variables|Default|SetMoveBackOnLeave false)
  (if (Variables|Default|GetStartOnContact)
    (Components|Timeline|SetPlayRate (Variables|Default|GetPlatformDriver) (/ 1.0 (Variables|Default|GetTimeToReachTarget)))
    (bind (_direction _0_1) (Timeline|PlatformDriver Play)
      (:Update
        (Transformation|SetRelativeLocation (Variables|Default|GetSM_PlatformBase) (Math|Vector|Lerp(Vector) "0, 0, 0" (Variables|Default|GetTarget) _0_1) false false))
      (:Finished
        (if (not (Variables|Default|GetMoveBackOnLeave))
          (if (Variables|Default|GetPlayInLoop)
            (switch Utilities|FlowControl|Switch|SwitchonETimelineDirection _direction
              (:Forward
                (CallFunction|ReverseinLoop))
              (:Backward
                (CallFunction|Replay)))))))))

(event OnComponentEndOverlap(Collision)
  (params (OverlappedComponent :type Primitive%20Component%20Object%20Reference) (OtherActor :type Actor%20Object%20Reference) (OtherComp :type Primitive%20Component%20Object%20Reference) (OtherBodyIndex :type Integer))
  (Variables|Default|SetMoveBackOnLeave true)
  (CallFunction|Reverse))

(event Custom|Replay
  (bind (_direction _0_1) (Timeline|PlatformDriver PlayFromStart)
    (:Update
      (Transformation|SetRelativeLocation (Variables|Default|GetSM_PlatformBase) (Math|Vector|Lerp(Vector) "0, 0, 0" (Variables|Default|GetTarget) _0_1) false false))
    (:Finished
      (if (not (Variables|Default|GetMoveBackOnLeave))
        (if (Variables|Default|GetPlayInLoop)
          (switch Utilities|FlowControl|Switch|SwitchonETimelineDirection _direction
            (:Forward
              (CallFunction|ReverseinLoop))
            (:Backward
              (CallFunction|Replay))))))))

(event Custom|ReverseInLoop
  (bind (_direction _0_1) (Timeline|PlatformDriver ReverseFromEnd)
    (:Update
      (Transformation|SetRelativeLocation (Variables|Default|GetSM_PlatformBase) (Math|Vector|Lerp(Vector) "0, 0, 0" (Variables|Default|GetTarget) _0_1) false false))
    (:Finished
      (if (not (Variables|Default|GetMoveBackOnLeave))
        (if (Variables|Default|GetPlayInLoop)
          (switch Utilities|FlowControl|Switch|SwitchonETimelineDirection _direction
            (:Forward
              (CallFunction|ReverseinLoop))
            (:Backward
              (CallFunction|Replay))))))))

(event Custom|Reverse
  (bind (_direction _0_1) (Timeline|PlatformDriver Reverse)
    (:Update
      (Transformation|SetRelativeLocation (Variables|Default|GetSM_PlatformBase) (Math|Vector|Lerp(Vector) "0, 0, 0" (Variables|Default|GetTarget) _0_1) false false))
    (:Finished
      (if (not (Variables|Default|GetMoveBackOnLeave))
        (if (Variables|Default|GetPlayInLoop)
          (switch Utilities|FlowControl|Switch|SwitchonETimelineDirection _direction
            (:Forward
              (CallFunction|ReverseinLoop))
            (:Backward
              (CallFunction|Replay))))))))

(event EventBeginPlay
  (|CallParentFunction)
  (if (not (Variables|Default|GetStartOnContact))
    (Components|Timeline|SetPlayRate (Variables|Default|GetPlatformDriver) (/ 1.0 (Variables|Default|GetTimeToReachTarget)))
    (bind (_direction _0_1) (Timeline|PlatformDriver Play)
      (:Update
        (Transformation|SetRelativeLocation (Variables|Default|GetSM_PlatformBase) (Math|Vector|Lerp(Vector) "0, 0, 0" (Variables|Default|GetTarget) _0_1) false false))
      (:Finished
        (if (not (Variables|Default|GetMoveBackOnLeave))
          (if (Variables|Default|GetPlayInLoop)
            (switch Utilities|FlowControl|Switch|SwitchonETimelineDirection _direction
              (:Forward
                (CallFunction|ReverseinLoop))
              (:Backward
                (CallFunction|Replay)))))))))

(fn ConstructionScript
  (|CallParentFunction))