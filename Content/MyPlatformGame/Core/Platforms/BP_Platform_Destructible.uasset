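; Destructible platform that breaks after accumulated time with something overlapping its trigger, then replaces itself with a fresh copy after a delay.
; Overlap starts camera shake, an emissive timeline and a break timer, which pauses when overlap ends.
; On break, the Geometry Collection simulates physics and receives radial strain and velocity fields.
; The construction script sizes trigger and collision boxes to the mesh and randomizes the dynamic material's color.
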(event OnComponentBeginOverlap(Trigger)
  (params (OverlappedComponent :type Primitive%20Component%20Object%20Reference) (OtherActor :type Actor%20Object%20Reference) (OtherComp :type Primitive%20Component%20Object%20Reference) (OtherBodyIndex :type Integer) (bFromSweep :type Boolean) (SweepResult :type Hit%20Result%20Structure%20%28by%20ref%29))
  (Components|Timeline|SetPlayRate (Variables|Default|GetEmissiveDriver) (/ 1.0 (Variables|Default|GetTimeUntilBreakEvent)))
  (Audio|Components|Audio|Play (Variables|Default|GetEmissiveDriver))
  (CameraShake|Start (Variables|Default|GetCameraShakeSource))
  (if (Utilities|Time|IsValidTimerHandle (Variables|Default|GetMyPlatformTimer))
    (Utilities|Time|UnpauseTimerbyHandle (Variables|Default|GetMyPlatformTimer))
    (else
      (bind _returnvalue (Utilities|Time|SetTimerbyEvent (delegate Custom|DestroyPlatform) (Variables|Default|GetTimeUntilBreakEvent)))
      (Variables|Default|SetMyPlatformTimer _returnvalue))))

(event OnComponentEndOverlap(Trigger)
  (params (OverlappedComponent :type Primitive%20Component%20Object%20Reference) (OtherActor :type Actor%20Object%20Reference) (OtherComp :type Primitive%20Component%20Object%20Reference) (OtherBodyIndex :type Integer))
  (Utilities|String|Reverse (Variables|Default|GetEmissiveDriver))
  (CameraShake|StopAllCameraShakes (Variables|Default|GetCameraShakeSource) true)
  (Audio|Components|Audio|Stop (Variables|Default|GetEmissiveDriver))
  (Utilities|Time|PauseTimerbyHandle (Variables|Default|GetMyPlatformTimer)))

(event Custom|DestroyPlatform
  (Physics|SetSimulatePhysics (Variables|Default|GetGC_DestructiblePlatform) true)
  (CallFunction|DestroyFunction)
  (Components|DestroyComponent (Variables|Default|GetTrigger))
  (Utilities|Time|SetTimerbyFunctionName 0 "Respawn" 3.0))

(event EventBeginPlay
  (|CallParentFunction) ; This node is disabled and will not be called.\nDrag off pins to build functionality.
)

(fn ConstructionScript
  (Utilities|FlowControl|Sequence
    (:then_0
      ;[0 0 0] Scale Trigger and Collision Boxes
      (Components|Box|SetBoxExtent (Variables|Default|GetTrigger) (.min (Components|StaticMesh|GetLocalBounds (Variables|Default|GetGC_DestructiblePlatform))) true))
    (:then_1
      ;[0 0 0] Set Dynamic Material
      (bind _returnvalue (Rendering|Material|CreateDynamicMaterialInstance (Variables|Default|GetGC_DestructiblePlatform) 0 "/Game/MyPlatformGame/Art/MaterialLibrary/Master/M_Color_Master.M_Color_Master" "None" :!class /Script/Engine.PrimitiveComponent))
      (bind _output_get (Variables|Default|SetMyDynamicMaterial _returnvalue))
      (Rendering|Material|SetVectorParameterValue _output_get "Color" (Math|Color|MakeColor (Math|Float|Clamp(Float) (Math|Random|RandomFloat) 0.0 0.5) (Math|Float|Clamp(Float) (Math|Random|RandomFloat) 0.0 0.5) (Math|Float|Clamp(Float) (Math|Random|RandomFloat) 0.0 0.5)) :!class /Script/Engine.MaterialInstanceDynamic)
      (Rendering|Material|SetVectorParameterValue (Variables|Default|GetMyDynamicMaterial) "EmissiveColor" "(R=0.000000,G=0.000000,B=0.000000,A=1.000000)" :!class /Script/Engine.MaterialInstanceDynamic))))

(fn DestroyFunction
  (bind _gc_destructibleplatform (Variables|Default|GetGC_DestructiblePlatform))
  (bind (_origin _boxextent _sphereradius) (Collision|GetComponentBounds _gc_destructibleplatform))
  (Class|FieldSystemComponent|ApplyPhysicsField (Variables|Default|GetFieldSystem) true "Field_ExternalClusterStrain" 0 (Field|SetRadialFalloff (Variables|Default|GetRadialFalloff) 5e+05 0.0 1.0 0.0 _sphereradius _origin "Field_FallOff_None"))
  (Class|FieldSystemComponent|ApplyPhysicsField (Variables|Default|GetFieldSystem) true "Field_LinearVelocity" 0 (Field|SetRadialVector (Variables|Default|GetRadialVector) 1e+03 (.Origin (Collision|GetComponentBounds (Variables|Default|GetGC_DestructiblePlatform))))))

(fn Respawn
  (Game|SpawnActorfromClass "BP_Platform_Destructible_C" (Transformation|GetActorTransform) "AlwaysSpawn" "MultiplyWithRoot" 0 0)
  (Actor|DestroyActor))